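; EnemyBP is an enemy character that hurts a Bomberman on contact and tints its body with a configurable color.
; A capsule hit applies fixed damage through the Bomberman's DamageComponent, using ToBomberman to filter out other EnemyBP actors.
; UpdateColor runs at construction and BeginPlay, creating a dynamic material instance to set BodyColor on the mesh.
; An IsBomberman check is defined but unused here.
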(event OnComponentHit(CapsuleComponent)
  (params (HitComponent :type Primitive%20Component%20Object%20Reference) (OtherActor :type Actor%20Object%20Reference) (OtherComp :type Primitive%20Component%20Object%20Reference) (NormalImpulse :type Vector :default "0, 0, 0") (Hit :type Hit%20Result%20Structure%20%28by%20ref%29))
  (bind _bomberman (CallFunction|ToBomberman OtherActor))
  (Utilities|IsValid _bomberman
    (:Is%20Valid
      (Class|DamageComponent|ApplyDamage (Variables|/Script/Bomberman.BombermanCharacter|GetDamageComponent _bomberman) 5e+01))))

(event EventBeginPlay
  (|CallParentFunction)
  (CallFunction|UpdateColor (Variables|Default|GetColor)))

(event Collision|EventActorBeginOverlap
  (params (OtherActor :type Actor%20Object%20Reference))
  (|CallParentFunction OtherActor) ; This node is disabled and will not be called.\nDrag off pins to build functionality.
)

(event EventTick
  (params (DeltaSeconds :type Float%20%28single-precision%29))
  (|CallParentFunction DeltaSeconds) ; This node is disabled and will not be called.\nDrag off pins to build functionality.
)

(fn ConstructionScript
  (|CallParentFunction)
  (CallFunction|UpdateColor (Variables|Default|GetColor)))

(fn UpdateColor
  (params (Color :type Linear%20Color%20Structure))
  (bind _returnvalue (Rendering|Material|CreateDynamicMaterialInstance (Variables|Character|GetMesh) 0 0 "None" :!class /Script/Engine.PrimitiveComponent))
  (bind _output_get (LocalVariables|SetLBodyMaterial _returnvalue))
  (Rendering|Material|SetVectorParameterValue _output_get "BodyColor" Color :!class /Script/Engine.MaterialInstanceDynamic)
  (Rendering|Material|SetMaterial (Variables|Character|GetMesh) 0 (LocalVariables|GetLBodyMaterial))
  (return))

(fn IsBomberman
  (params (Actor :type Actor%20Object%20Reference))
  (Utilities|FlowControl|Sequence
    (:then_0
      (bind _asbomberman_bp (Utilities|Casting|CastToBombermanBP Actor)))
    (:then_1
      (bind _asenemy_bp (Utilities|Casting|CastToEnemyBP Actor)))
    (:then_2
      (return (and (Utilities|IsValid _asbomberman_bp) (not (Utilities|IsValid _asenemy_bp)))))))

(fn ToBomberman
  (params (Actor :type Actor%20Object%20Reference))
  (Utilities|Casting|CastToEnemyBP Actor
    (:then
      _)
    (:CastFailed
      (bind _asbomberman_bp (Utilities|Casting|CastToBombermanBP Actor)
        (:then
          (LocalVariables|SetLBomberman _asbomberman_bp))
        (:CastFailed
          _))))
  (return (LocalVariables|GetLBomberman)))