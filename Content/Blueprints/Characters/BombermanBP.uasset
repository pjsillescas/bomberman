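; Bomberman character Blueprint, used for both player and AI, that handles death and creates the main HUD.
; On BeginPlay it binds a destroy handler on its DamageComponent and adds the HUD to the viewport.
; Player death blends the camera to a child actor, then takes a life through BombermanGameInstance after a delay.
; AI death detaches the controller, then destroys the actor after a delay.
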(event Custom|OnDestroy
  (if (CallFunction|IsPlayer)
    (CallFunction|DestroyPlayerCharacter)
    (else
      (CallFunction|DestroyAICharacter))))

(event Custom|DestroyAICharacter
  (Class|Pawn|DetachfromControllerPendingDestroy)
  (Utilities|FlowControl|Delay 5.0)
  (Actor|DestroyActor))

(event Custom|DestroyPlayerCharacter
  (CallFunction|GameOver)
  (Utilities|FlowControl|Delay 6.0)
  (bind _asbomberman_game_instance (Utilities|Casting|CastToBombermanGameInstance (Game|GetGameInstance)))
  (Class|BombermanGameInstance|TakeLife _asbomberman_game_instance))

(event EventBeginPlay
  (Class|DamageComponent|SetonDestroy (Variables|Default|GetDamageComponent) (EventDispatchers|CreateEvent :!event Custom|OnDestroy))
  (bind _returnvalue (UserInterface|CreateWidget "/Game/Blueprints/UI/MainHUD.MainHUD_C" (Game|GetPlayerController 0)))
  (UserInterface|Viewport|AddtoViewport _returnvalue 0))

(event Collision|EventActorBeginOverlap
  (params (OtherActor :type Actor%20Object%20Reference)))

(event EventTick
  (params (DeltaSeconds :type Float%20%28single-precision%29)))

(fn ConstructionScript)

(fn GameOver
  (Game|Player|SetViewTargetwithBlend (Game|GetPlayerController 0) (Variables|/Script/Engine.ChildActorComponent|GetChildActor (Variables|Default|GetChildActor)) 3.0 "VTBlend_Linear" 0.0 false)
  (return))

(fn IsPlayer
  (return (Class|Controller|IsPlayerController (Pawn|GetController))))